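; Build-mode component that lets the player preview and place a floodlight in the world.
; While building, Tick traces 10 meters from the player's face along control rotation and moves a preview-material mesh to the hit location.
; A DoOnce creates the preview, showing a battery unit mesh, and resets when building ends.
; Inputs toggle build mode, rotate by 90 degrees, or spawn BP_Floodlight at the preview transform and exit.
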(event `Preview Loop`
  (bind _returnvalue (`SceneComponent.K2_GetComponentLocation` (`/Game/Blueprints/BP_fpsController.Face` (`self.Player`))))
  (bind _outhit (`KismetSystemLibrary.LineTraceSingleForObjects` _returnvalue (+ _returnvalue (* (`KismetMathLibrary.GetForwardVector` (`Pawn.GetControlRotation` (`self.Player`))) 1000.0)) (`|MakeArray` "ObjectTypeQuery1" :!type "EObjectTypeQuery Enum")))
  (`|ExecutionSequence`
    (:`then_0`
      (`/Engine/EditorBlueprintResources/StandardMacros.DoOnce` false :!label _label
        (:`Completed`
          (`self.StartBuildPreview` (`self.Player`)))))
    (:`then_1`
      (bind _output_get (set `self.Build Preview Location` (`KismetMathLibrary.MakeTransform` (`.Location` (`GameplayStatics.BreakHitResult` _outhit)) (`self.Build Preview Location Rotation`))))
      (`SceneComponent.K2_SetWorldTransform` (`self.Preview Mesh`) (`KismetMathLibrary.MakeTransform` (.location _output_get) (`self.Build Preview Location Rotation`)) false false))))

(event `ResetBuildNode`
  (goto _label :!via `Reset`))

(event `self.ReceiveTick`
  (params (DeltaSeconds :type "Float (single-precision)"))
  (if (`self.Is Building`)
    (`self.Preview Loop`)))

(event `EnhancedInput|/Game/Input/BUILD_IA`
  (params (ActionValue :type Boolean) (ElapsedSeconds :type "Float (double-precision)") (TriggeredSeconds :type "Float (double-precision)") (InputAction :type "InputAction Object Reference" :default "/Game/Input/BUILD_IA.BUILD_IA"))
  (:`Started`
    (bind _output_get (set `self.Is Building` (not (`self.Is Building`))))
    (if (not _output_get)
      (`StaticMeshComponent.SetStaticMesh` (`self.Preview Mesh`) null)
      (set `self.Preview Mesh` null)
      (`self.ResetBuildNode`))))

(event `EnhancedInput|/Game/Input/INTERACT_IA`
  (params (ActionValue :type Boolean) (ElapsedSeconds :type "Float (double-precision)") (TriggeredSeconds :type "Float (double-precision)") (InputAction :type "InputAction Object Reference" :default "/Game/Input/INTERACT_IA.INTERACT_IA"))
  (:`Started`
    (if (`self.Is Building`)
      (`self.PlaceBuildObject`)
      (set `self.Is Building` false)
      (`StaticMeshComponent.SetStaticMesh` (`self.Preview Mesh`) null)
      (set `self.Preview Mesh` null)
      (`self.ResetBuildNode`))))

(event `EnhancedInput|/Game/Input/ROTATE_IA`
  (params (ActionValue :type Boolean) (ElapsedSeconds :type "Float (double-precision)") (TriggeredSeconds :type "Float (double-precision)") (InputAction :type "InputAction Object Reference" :default "/Game/Input/ROTATE_IA.ROTATE_IA"))
  (bind _build_preview_location (`self.Build Preview Location`))
  (:`Started`
    (set `self.Build Preview Location Rotation` (`KismetMathLibrary.MakeRotator` 0.0 0.0 (+ (.yaw (.rotation (`self.Build Preview Location`))) 90.0)))
    (set `self.Build Preview Location` (`KismetMathLibrary.MakeTransform` (.location _build_preview_location) (`KismetMathLibrary.MakeRotator` 0.0 0.0 (+ (.yaw (.rotation _build_preview_location)) 90.0))))
    (`KismetSystemLibrary.PrintString` "Hello")))

(fn `PlaceBuildObject`
  (bind (_build_preview_location_location _build_preview_location_rotation) (`KismetMathLibrary.BreakTransform` (`self.Build Preview Location`)))
  (`|SpawnActorFromClass` "/Game/Objects/BP_Floodlight.BP_Floodlight_C" (`KismetMathLibrary.MakeTransform` _build_preview_location_location _build_preview_location_rotation) "Undefined" "MultiplyWithRoot" null null))

(fn `StartBuildPreview`
  (params (player :type "/Game/Blueprints/BP_fpsController Object Reference"))
  (`|ExecutionSequence`
    (:`then_0`
      (set `self.Player` player))
    (:`then_1`
      (bind _returnvalue (`|AddComponentByClass` (`self.Player`) "/Script/Engine.StaticMeshComponent" false (`self.Build Preview Location`)))
      (bind _output_get (set `self.Preview Mesh` _returnvalue))
      (`StaticMeshComponent.SetStaticMesh` _output_get "/Game/Sci_Fi_Light/Static_Meshes/SM_Sci_Fi_Battery_Unit/Mesh/SM_Sci_Fi_Battery_Unit.SM_Sci_Fi_Battery_Unit")
      (`PrimitiveComponent.SetMaterial` (`self.Preview Mesh`) 0 "/Game/Materials/M_BuildPreview.M_BuildPreview"))))