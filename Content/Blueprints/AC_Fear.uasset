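; AC_Fear is an actor component that tracks a fear level clamped between 0 and 100.
; Each tick it lowers fear while InSafeZone is set, otherwise it raises it by FearChangeRate scaled by delta time.
; ChangeFearRate sets a slower rise when the torch is on and a faster one when off, printing debug strings.
; Fear decay uses a fixed rate, independent of the torch.
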(event `self.ReceiveTick`
  (params (DeltaSeconds :type "Float (single-precision)"))
  (if (`self.inSafeZone`)
    (`self.decreaseFear` DeltaSeconds)
    (else
      (`self.IncreaseFear` DeltaSeconds))))

(fn `changeFearRate`
  (params (torchOn :type Boolean))
  (if torchOn
    (set `self.fearChangeRate` 1.0)
    (`KismetSystemLibrary.PrintString` "TORCH ON")
    (else
      (set `self.fearChangeRate` 3.0)
      (`KismetSystemLibrary.PrintString` "TORCH OFF"))))

(fn `decreaseFear`
  (params (deltaTime :type "Float (double-precision)"))
  (bind _output_get (set `self.currentFearLevel` (`KismetMathLibrary.FClamp` (- (`self.currentFearLevel`) (* deltaTime 1.0)) 0.0 100.0))))

(fn `IncreaseFear`
  (params (deltaTime :type "Float (double-precision)"))
  (bind _output_get (set `self.currentFearLevel` (`KismetMathLibrary.FClamp` (+ (`self.currentFearLevel`) (* deltaTime (`self.fearChangeRate`))) 0.0 100.0))))