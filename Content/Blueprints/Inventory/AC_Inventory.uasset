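; Inventory component that stores items in a map from ID to an item struct holding data and quantity.
; Give adds Quantity to an existing stack, or stores the passed item as-is for a new ID, printing debug totals.
; CheckInventory prints each item's name and quantity.
; SearchInventory returns true only when the item exists with exactly the requested quantity, not at least that amount.
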(fn `checkInventory`
  (bind (_keypin _valuepin) (`|MapForEach` (`self.items`))
    (:`then`
      (bind (_itemdata _quantity) (break `InventoryItem` _valuepin))
      (`KismetSystemLibrary.PrintString` (`KismetStringLibrary.Concat_StrStr` "Name: " (`KismetTextLibrary.Conv_TextToString` (`ItemDataAsset.Name` _itemdata)) "   " "Quantity: " (`KismetStringLibrary.Conv_IntToString` _quantity))))
    (:`CompletedPin`
      (`KismetSystemLibrary.PrintString` "Done"))))

(fn `Give`
  (params (ID :type Name) (Quantity :type Integer :default -1) (GiveItem :type "InventoryItem Structure"))
  (bind _items (`self.items`))
  (bind (_value _returnvalue) (`BlueprintMapLibrary.Map_Find` _items ID))
  (`|ExecutionSequence`
    (:`then_0`
      (set `self.Item` GiveItem)
      (if _returnvalue
        (bind _structout (setmembers `InventoryItem` :`StructRef` _value))
        (bind _returnvalue_2 (+ (`.Quantity` (break `InventoryItem` _structout)) Quantity))
        (set `self.Item` (make `InventoryItem` (break `InventoryItem` _structout) _returnvalue_2))
        (`KismetSystemLibrary.PrintString` (`KismetStringLibrary.Concat_StrStr` "Old Quantity: " (`KismetStringLibrary.Conv_IntToString` (`.Quantity` (break `InventoryItem` _structout))) " New Quantity: " (`KismetStringLibrary.Conv_IntToString` _returnvalue_2)))))
    (:`then_1`
      (bind _output_get (set `self.items` _items))
      (`BlueprintMapLibrary.Map_Add` _output_get ID (`self.Item`)))
    (:`then_2`
      (`|MapForEach` (`self.items`)
        (:`then`
          (`KismetSystemLibrary.PrintString` (`KismetStringLibrary.Concat_StrStr` "Final quantity: " (`KismetStringLibrary.Conv_IntToString` (`.Quantity` (break `InventoryItem` (`self.Item`)))))))))))

(fn `searchInventory`
  (params (item :type Name) (quantity :type Integer :default 1))
  (returns (doesExist :type Boolean))
  (bind (_value _returnvalue) (`BlueprintMapLibrary.Map_Find` (`self.items`) item))
  (if _returnvalue
    (if (== (`.Quantity` (break `InventoryItem` _value)) quantity)
      (return true)
      (else
        (return false)))))