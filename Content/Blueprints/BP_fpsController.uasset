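; First-person player character that handles movement, look, jump, crouch, sprint/walk speeds, a torch and interaction through Enhanced Input.
; BeginPlay adds the mapping context and creates the Fear, Inventory and BuildSystem components.
; A short per-tick line trace supplies the interact target: pickups go to Inventory, and cave entrances open if an inventory search finds Entrance Switches.
; The torch spotlight follows control rotation, and toggling it updates the fear rate.
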(event `self.ReceiveBeginPlay`
  ; Add input controls
  (bind _asplayer_controller (cast `PlayerController` (`self.GetController`)))
  (bind _returnvalue (pcsubsystem `EnhancedInputLocalPlayerSubsystem` _asplayer_controller))
  (`/Engine/EditorBlueprintResources/StandardMacros.IsValid` _returnvalue
    (:`Is Valid`
      (`EnhancedInputSubsystemInterface.AddMappingContext` _returnvalue "/Game/Input/FPS_IMC.FPS_IMC" 0 (struct))
      (bind _returnvalue_2 (`AddComponent|NODE_AddAC_Fear-0`))
      (set `self.Fear` _returnvalue_2)
      (bind _returnvalue_3 (`AddComponent|NODE_AddAC_Inventory-0`))
      (set `self.Inventory` _returnvalue_3)
      (set `self.CrouchedEyeHeight` 60.0)
      (bind _returnvalue_4 (`AddComponent|NODE_AddAC_BuildMode-2`))
      (bind _output_get (set `self.BuildMode` _returnvalue_4))
      (set `/Game/Blueprints/AC_BuildSystem.Player` self _output_get))))

(event `EnhancedInput|/Game/Input/MOVE_IA`
  (params (ActionValue :type "Vector2D Structure") (ElapsedSeconds :type "Float (double-precision)") (TriggeredSeconds :type "Float (double-precision)") (InputAction :type "InputAction Object Reference" :default "/Game/Input/MOVE_IA.MOVE_IA"))
  (:`Triggered`
    (`self.AddMovementInput` (`self.GetActorRightVector`) ActionValue_X)
    (`self.AddMovementInput` (`self.GetActorForwardVector`) ActionValue_Y)))

(event `EnhancedInput|/Game/Input/SPRINT_IA`
  (params (ActionValue :type Boolean) (ElapsedSeconds :type "Float (double-precision)") (TriggeredSeconds :type "Float (double-precision)") (InputAction :type "InputAction Object Reference" :default "/Game/Input/SPRINT_IA.SPRINT_IA"))
  (bind _charactermovement (`self.CharacterMovement`))
  (:`Triggered`
    (set `CharacterMovementComponent.MaxWalkSpeed` 900.0 _charactermovement)
    (set `CharacterMovementComponent.MaxWalkSpeedCrouched` 400.0 _charactermovement))
  (:`Completed`
    (set `CharacterMovementComponent.MaxWalkSpeed` 600.0 _charactermovement)
    (set `CharacterMovementComponent.MaxWalkSpeedCrouched` 300.0 _charactermovement)))

(event `EnhancedInput|/Game/Input/PICKUP_IA`
  (params (ActionValue :type Boolean) (ElapsedSeconds :type "Float (double-precision)") (TriggeredSeconds :type "Float (double-precision)") (InputAction :type "InputAction Object Reference" :default "/Game/Input/PICKUP_IA.PICKUP_IA"))
  (:`Completed`
    (bind (_bblockinghit _binitialoverlap _time _distance _location _impactpoint _normal _impactnormal _physmat _hitactor) (`GameplayStatics.BreakHitResult` (stale `self.ReceiveTick` _outhit)))
    (bind _asbp_pickup_object (cast `/Game/Blueprints/Inventory/BP_PickupObject` _hitactor)
      (:`then`
        (bind (_givenitem _itemid _quantity) (`/Game/Blueprints/Inventory/AC_Interactable.Pickup` (`/Game/Blueprints/Inventory/BP_PickupObject.AC_Interactable` _asbp_pickup_object) (`/Game/Blueprints/Inventory/BP_PickupObject.giveItem` _asbp_pickup_object) _asbp_pickup_object))
        (`/Game/Blueprints/Inventory/AC_Inventory.Give` (`self.Inventory`) _itemid _quantity _givenitem))
      (:`CastFailed`
        (bind _asbp_cave_entrance (cast `/Game/Blueprints/BP_caveEntrance` _hitactor)
          (:`then`
            (bind _doesexist (`/Game/Blueprints/Inventory/AC_Inventory.searchInventory` (`self.Inventory`) "Entrance Switch" 2))
            (if _doesexist
              (`/Game/Blueprints/BP_caveEntrance.OpenDoor` _asbp_cave_entrance)))
          (:`CastFailed`
            (`KismetSystemLibrary.PrintString` "Not Interactabe")))))))

(event `self.ReceiveTick`
  (params (DeltaSeconds :type "Float (single-precision)"))
  (bind _returnvalue (`SceneComponent.K2_GetComponentLocation` (`self.Face`)))
  (bind _outhit (`KismetSystemLibrary.LineTraceSingleForObjects` _returnvalue (+ _returnvalue (* (`KismetMathLibrary.GetForwardVector` (`self.GetControlRotation`)) 200.0)) (`|MakeArray` "ObjectTypeQuery1" :!type "EObjectTypeQuery Enum"))))

(event `EnhancedInput|/Game/Input/LOOK_IA`
  (params (ActionValue :type "Vector Structure") (ElapsedSeconds :type "Float (double-precision)") (TriggeredSeconds :type "Float (double-precision)") (InputAction :type "InputAction Object Reference" :default "/Game/Input/LOOK_IA.LOOK_IA"))
  (:`Triggered`
    (`self.AddControllerYawInput` ActionValue_X)
    (`self.AddControllerPitchInput` ActionValue_Y)
    (`SceneComponent.K2_SetWorldRotation` (`self.SpotLight`) (`KismetMathLibrary.MakeRotator` 0.0 (.pitch (`self.GetControlRotation`)) (.yaw (`self.GetControlRotation`))) false false)))

(event `EnhancedInput|/Game/Input/WALK_IA`
  (params (ActionValue :type Boolean) (ElapsedSeconds :type "Float (double-precision)") (TriggeredSeconds :type "Float (double-precision)") (InputAction :type "InputAction Object Reference" :default "/Game/Input/WALK_IA.WALK_IA"))
  (bind _charactermovement (`self.CharacterMovement`))
  (:`Triggered`
    (set `CharacterMovementComponent.MaxWalkSpeed` 450.0 _charactermovement)
    (set `CharacterMovementComponent.MaxWalkSpeedCrouched` 150.0 _charactermovement))
  (:`Completed`
    (set `CharacterMovementComponent.MaxWalkSpeed` 600.0 _charactermovement)
    (set `CharacterMovementComponent.MaxWalkSpeedCrouched` 300.0 _charactermovement)))

(event `EnhancedInput|/Game/Input/JUMP_IA`
  (params (ActionValue :type Boolean) (ElapsedSeconds :type "Float (double-precision)") (TriggeredSeconds :type "Float (double-precision)") (InputAction :type "InputAction Object Reference" :default "/Game/Input/JUMP_IA.JUMP_IA"))
  (:`Triggered`
    (`self.Jump`))
  (:`Completed`
    (`self.StopJumping`)))

(event `EnhancedInput|/Game/Input/CROUCH_IA`
  (params (ActionValue :type Boolean) (ElapsedSeconds :type "Float (double-precision)") (TriggeredSeconds :type "Float (double-precision)") (InputAction :type "InputAction Object Reference" :default "/Game/Input/CROUCH_IA.CROUCH_IA"))
  (:`Started`
    (if (`NavMovementComponent.IsCrouching` (`self.CharacterMovement`))
      (`self.UnCrouch`)
      (else
        (`self.Crouch`)))
    (`KismetSystemLibrary.PrintString` (`KismetStringLibrary.Conv_BoolToString` (`self.CanCrouch`)))))

(event `EnhancedInput|/Game/Input/Inventory_IA`
  (params (ActionValue :type Boolean) (ElapsedSeconds :type "Float (double-precision)") (TriggeredSeconds :type "Float (double-precision)") (InputAction :type "InputAction Object Reference" :default "/Game/Input/Inventory_IA.Inventory_IA"))
  (:`Started`
    (`/Game/Blueprints/Inventory/AC_Inventory.checkInventory` (`self.Inventory`))))

(event `EnhancedInput|/Game/Input/TORCH_IA`
  (params (ActionValue :type Boolean) (ElapsedSeconds :type "Float (double-precision)") (TriggeredSeconds :type "Float (double-precision)") (InputAction :type "InputAction Object Reference" :default "/Game/Input/TORCH_IA.TORCH_IA"))
  (:`Completed`
    (`SceneComponent.ToggleVisibility` (`self.SpotLight`) false)
    (bind _output_get (set `self.torchActive` (`SceneComponent.bVisible` (`self.SpotLight`))))
    (`AC_Fear.ChangeFearRate` (`self.Fear`) _output_get)))

(fn `UserConstructionScript`)